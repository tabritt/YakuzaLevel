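; BP_Put is a pot actor that can be picked up and damages enemies on contact.
; Interact prints a debug message, triggers a short delayed self-destroy and returns the Pot's static mesh to the caller.
; When its Collider overlaps a BP_Enemy, it applies fixed damage, destroys itself, then subtracts the returned damage from EnemyHealth and prints the result.
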(event OnComponentBeginOverlap(Collider)
  (params (OverlappedComponent :type Primitive%20Component%20Object%20Reference) (OtherActor :type Actor%20Object%20Reference) (OtherComp :type Primitive%20Component%20Object%20Reference) (OtherBodyIndex :type Integer) (bFromSweep :type Boolean) (SweepResult :type Hit%20Result%20Structure%20%28by%20ref%29))
  (bind _asbp_enemy (Utilities|Casting|CastToBP_Enemy OtherActor))
  (bind _returnvalue (Game|Damage|ApplyDamage _asbp_enemy 2e+01 0 0))
  (Actor|DestroyActor)
  (Variables|/Game/AI/BP_Enemy.BP_Enemy_C|SetEnemyHealth _asbp_enemy (- (Variables|/Game/AI/BP_Enemy.BP_Enemy_C|GetEnemyHealth _asbp_enemy) _returnvalue))
  (Development|PrintString (Utilities|String|ToString(Float) (Variables|/Game/AI/BP_Enemy.BP_Enemy_C|GetEnemyHealth _asbp_enemy))))

(event Custom|E_DestroyActor
  (Utilities|FlowControl|Delay 0.2)
  (Actor|DestroyActor))

(fn ConstructionScript)

(fn Interact
  (params (NewParam :type Static%20Mesh%20Object%20Reference))
  (Development|PrintString "picking")
  (CallFunction|EDestroyActor)
  (return (Variables|/Script/Engine.StaticMeshComponent|GetStaticMesh (Variables|Default|GetPot))))