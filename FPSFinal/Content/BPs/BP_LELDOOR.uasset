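; BP_LELDOOR is a moving door, apparently for an elevator, that slides aside along X, rises on Z, then slides back.
; An ALS_AnimMan character overlapping its Box trigger starts the sequence, which DoOnce limits to a single run.
; Chained Delay and MoveComponentTo nodes move the root component, with one-shot VInterpTo calls on actor location supplying targets that effectively equal the full offsets.
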(event OnComponentBeginOverlap(Box)
  (params (OverlappedComponent :type Primitive%20Component%20Object%20Reference) (OtherActor :type Actor%20Object%20Reference) (OtherComp :type Primitive%20Component%20Object%20Reference) (OtherBodyIndex :type Integer) (bFromSweep :type Boolean) (SweepResult :type Hit%20Result%20Structure%20%28by%20ref%29))
  (bind _returnvalue (Transformation|GetActorLocation))
  (bind _returnvalue_2 (Transformation|GetActorLocation))
  (bind _returnvalue_3 (Transformation|GetActorLocation))
  (Utilities|Casting|CastToALS_AnimMan_CharacterBP OtherActor)
  (Utilities|FlowControl|DoOnce false
    (:Completed
      (Utilities|FlowControl|Delay 2.0)
      (Components|MoveComponentTo (Variables|Default|GetDefaultSceneRoot) (Math|Interpolation|VInterpTo _returnvalue_2 (+ _returnvalue_2 "-300.000000,0.000000,0.000000") 2.0 7.0) (Transformation|GetActorRotation) false false 3.0 false)
      (Utilities|FlowControl|Delay 1.0)
      (Components|MoveComponentTo (Variables|Default|GetDefaultSceneRoot) (Math|Interpolation|VInterpTo _returnvalue_3 (+ _returnvalue_3 "0.000000,0.000000,932.000000") 3.0 2.0) (Transformation|GetActorRotation) false false 4.0 false)
      (Utilities|FlowControl|Delay 0.5)
      (Components|MoveComponentTo (Variables|Default|GetDefaultSceneRoot) (Math|Interpolation|VInterpTo _returnvalue (+ _returnvalue "300.000000,0.000000,0.000000") 2.0 7.0) (Transformation|GetActorRotation) false false 3.0 false))))

(fn ConstructionScript)