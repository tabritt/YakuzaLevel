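; BP_Door1 is an interactable door Blueprint with two door components, Door1 and Door2.
; Interact toggles the DoorOpen flag and plays or reverses the DoorRotation timeline.
; Rotation setters map separate timeline tracks to each door's yaw, but neither is connected to execution, so this graph never applies the rotation.
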(event EventInteract
  (if (not (Variables|Default|GetDoorOpen))
    (Variables|Default|SetDoorOpen true)
    (bind (_direction _door1rotate _door2rotate) (Timeline|DoorRotation Play))
    (else
      (Variables|Default|SetDoorOpen false)
      (Timeline|DoorRotation Reverse))))

(fn ConstructionScript
  (|CallParentFunction))