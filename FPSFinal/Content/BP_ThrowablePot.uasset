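; BP_ThrowablePot is a pot actor that can be picked up; despite its name, it contains no throwing logic.
; Its construction script applies the ItemAttached mesh to the Pot component.
; Any overlap with the Sphere sets CanBePicked through a branch hardwired to true, and nothing clears it on exit.
; The Pickup event prints a debug message and destroys the actor without checking that flag.
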(event OnComponentBeginOverlap(Sphere)
  (params (OverlappedComponent :type Primitive%20Component%20Object%20Reference) (OtherActor :type Actor%20Object%20Reference) (OtherComp :type Primitive%20Component%20Object%20Reference) (OtherBodyIndex :type Integer) (bFromSweep :type Boolean) (SweepResult :type Hit%20Result%20Structure%20%28by%20ref%29))
  (Development|PrintString "in radius")
  (if true
    (Variables|Default|SetcanBePicked true)
    (Development|PrintString "pick up is true")
    (else
      (Variables|Default|SetcanBePicked false)
      (Development|PrintString "pick up is false"))))

(event EventBeginPlay)

(event Collision|EventActorBeginOverlap
  (params (OtherActor :type Actor%20Object%20Reference)))

(event EventTick
  (params (DeltaSeconds :type Float%20%28single-precision%29)))

(event EventPickup
  (Development|PrintString "Pick me up")
  (Actor|DestroyActor))

(fn ConstructionScript
  (Components|StaticMesh|SetStaticMesh (Variables|Default|GetPot) (Variables|Default|GetItemAttached)))