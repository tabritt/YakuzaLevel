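; BP_Range_Enemy is a ranged AI enemy that attacks the player character when pawn sensing spots it.
; On sight it sets the "hasSeenPlayer?" blackboard key, turns toward the player and, if able, spawns a BP_Shoot projectile.
; The projectile's impulse is its world location scaled up, not an aim vector, and damage is applied directly on firing.
; A CanAttack flag with a one-second delay limits the fire rate.
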(event OnSeePawn(PawnSensing)
  (params (Pawn :type Pawn%20Object%20Reference))
  ;[1 1 1] AI FINDS YOU
  (bind _asals_anim_man_character_bp (Utilities|Casting|CastToALS_AnimMan_CharacterBP Pawn))
  (AI|Components|Blackboard|SetValueasBool (AI|GetBlackboard (AI|GetAIController self)) (Utilities|Name|MakeLiteralName "hasSeenPlayer?") true)
  (Transformation|SetActorRotation (Math|Rotator|FindRelativeLookatRotation (Math|Conversions|ToTransform(Vector) (Transformation|GetActorLocation)) (Transformation|GetActorLocation _asals_anim_man_character_bp)))
  (if (Variables|Default|GetCanAttack?)
    (bind _returnvalue (Game|SpawnActorfromClass "/Game/BPs/BP_Shoot.BP_Shoot_C" (Transformation|GetWorldTransform (Variables|Default|GetSpawnProjectileLocation)) "Undefined" "MultiplyWithRoot" 0 0))
    (Physics|AddImpulse (Variables|/Game/BPs/BP_Shoot.BP_Shoot_C|GetCapsule _returnvalue) (* (Transformation|GetWorldLocation (Variables|/Game/BPs/BP_Shoot.BP_Shoot_C|GetCapsule _returnvalue)) 1e+02) "None" false)
    (Game|Damage|ApplyDamage _asals_anim_man_character_bp 1.0 0 0)
    (Variables|Default|SetCanAttack? false)
    (Utilities|FlowControl|Delay 1.0)
    (Variables|Default|SetCanAttack? true)))

(fn ConstructionScript
  (|CallParentFunction))