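; Melee enemy AI Blueprint that reacts when its PawnSensing component spots an ALS player character.
; On sighting, it sets the "hasSeenPlayer?" blackboard flag on its AI controller and calls the attack-player event.
; A short forward sphere trace against pawns then gates an attack montage and damage call when it hits the player.
; A CanAttack flag is switched off and restored after a brief delay, though this graph never checks it.
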(event OnSeePawn(PawnSensing)
  (params (Pawn :type Pawn%20Object%20Reference))
  (bind _returnvalue (Transformation|GetActorLocation))
  ;[1 1 1] AI FINDS YOU
  (Utilities|Casting|CastToALS_AnimMan_CharacterBP Pawn)
  (AI|Components|Blackboard|SetValueasBool (AI|GetBlackboard (AI|GetAIController self)) (Utilities|Name|MakeLiteralName "hasSeenPlayer?") true)
  (CallFunction|EAttackplayer)
  (bind (_outhit _returnvalue_2) (Collision|SphereTraceForObjects _returnvalue (+ _returnvalue (* (Math|Vector|GetForwardVector (Transformation|GetActorRotation)) 2.5e+02)) 0.0 (Utilities|Array|MakeArray "ObjectTypeQuery3") false 0 "ForDuration"))
  (if _returnvalue_2
    (Utilities|Casting|CastToALS_AnimMan_CharacterBP (.HitActor (Collision|BreakHitResult _outhit)))
    (Animation|PlayAnimMontage 0 1.0 "None")
    (Game|Damage|ApplyDamage 0 5.0 0 0)
    (Variables|Default|SetCanAttack? false)
    (Utilities|FlowControl|Delay 2.0)
    (Variables|Default|SetCanAttack? true)))

(fn ConstructionScript
  (|CallParentFunction))