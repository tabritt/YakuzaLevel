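; BP_Elevator is an elevator that rises once when an ALS_AnimMan_CharacterBP character enters its trigger.
; Overlapping ElevatorTrigger starts a four-second delay, then a DoOnce that is never reset prints a debug message and starts the move.
; MoveComponentTo raises the root component a fixed height over four seconds, using a one-shot VInterpTo call for the target, with no return trip.
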(event OnComponentBeginOverlap(ElevatorTrigger)
  (params (OverlappedComponent :type Primitive%20Component%20Object%20Reference) (OtherActor :type Actor%20Object%20Reference) (OtherComp :type Primitive%20Component%20Object%20Reference) (OtherBodyIndex :type Integer) (bFromSweep :type Boolean) (SweepResult :type Hit%20Result%20Structure%20%28by%20ref%29))
  (Utilities|Casting|CastToALS_AnimMan_CharacterBP OtherActor)
  (Utilities|FlowControl|Delay 4.0)
  (Utilities|FlowControl|DoOnce false
    (:Completed
      (Development|PrintString "in elevator")
      (Components|MoveComponentTo (Variables|Transformation|GetRootComponent) (Math|Interpolation|VInterpTo (Transformation|GetActorLocation) (+ (Transformation|GetActorLocation) "0.000000,0.000000,932.000000") 3.0 2.0) (Transformation|GetActorRotation) false false 4.0 false))))

(event EventBeginPlay)

(event EventTick
  (params (DeltaSeconds :type Float%20%28single-precision%29)))

(fn ConstructionScript)